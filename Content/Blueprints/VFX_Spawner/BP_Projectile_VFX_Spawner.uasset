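; Spawner actor that repeatedly fires BP_ProjectileMaster projectiles carrying configurable Niagara muzzle, projectile and hit impact effects.
; On BeginPlay it spawns one immediately, then a looping timer spawns more at ProjectileSpawnGap intervals from the actor's location.
; After each spawn it passes its effect assets, offset, destroy delay and decoration loop duration to the projectile, and sets velocity along fixed +X, scaled by ProjectileSpeed.
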(event Custom|SpawnProjectileVFX
  (bind _returnvalue (Game|SpawnActorfromClass "/Game/Blueprints/VFX_Spawner/BP_ProjectileMaster.BP_ProjectileMaster_C" (Math|Transform|MakeTransform (Transformation|GetActorLocation) "0, 0, 0" "1.000000,1.000000,1.000000") "Undefined" "MultiplyWithRoot" 0 0))
  (bind _output_get (Variables|Default|SetSpawnedProjectile _returnvalue))
  (Utilities|IsValid _output_get
    (:Is%20Valid
      (Utilities|FlowControl|Sequence
        (:then_0
          ;[0.2468 0 0.4531] Set VFX Niagara Variables
          (Variables|/Game/Blueprints/VFX_Spawner/BP_ProjectileMaster.BP_ProjectileMaster_C|SetMuzzleVFX (Variables|Default|GetSpawnedProjectile) (Variables|Default|GetMuzzleVFX))
          (Class|NiagaraComponent|SetAsset (Variables|/Game/Blueprints/VFX_Spawner/BP_ProjectileMaster.BP_ProjectileMaster_C|GetProjectileVFXComponent (Variables|Default|GetSpawnedProjectile)) (Variables|Default|GetMainProjectileVFX) true)
          (Variables|/Game/Blueprints/VFX_Spawner/BP_ProjectileMaster.BP_ProjectileMaster_C|SetHitImpactVFX (Variables|Default|GetSpawnedProjectile) (Variables|Default|GetHit%20ImpactVFX)))
        (:then_1
          ;[0.2468 0 0.4531] Set Projectile Speed
          (Variables|/Script/Engine.MovementComponent|SetVelocity (Variables|/Game/Blueprints/VFX_Spawner/BP_ProjectileMaster.BP_ProjectileMaster_C|GetProjectileVFXMovementComp (Variables|Default|GetSpawnedProjectile)) (* (Variables|Default|GetProjectileSpeed) "1.000000,0.000000,0.000000")))
        (:then_2
          (Variables|/Game/Blueprints/VFX_Spawner/BP_ProjectileMaster.BP_ProjectileMaster_C|SetMuzzleHitImpactSpawnOffset (Variables|Default|GetSpawnedProjectile) (Variables|Default|GetMuzzleHitImpactSpawnOffset))
          (Variables|/Game/Blueprints/VFX_Spawner/BP_ProjectileMaster.BP_ProjectileMaster_C|SetProjectileDestroyDelay (Variables|Default|GetSpawnedProjectile) (Variables|Default|GetProjectileDestroyDelay))
          (Niagara|SetNiagaraVariable(Float) (Variables|/Game/Blueprints/VFX_Spawner/BP_ProjectileMaster.BP_ProjectileMaster_C|GetProjectileVFXComponent (Variables|Default|GetSpawnedProjectile)) "DecorationParticlesLoopDuration" (Variables|Default|GetDecorationParticlesLoopDuration)))))))

(event EventBeginPlay
  (CallFunction|SpawnProjectileVFX)
  (Utilities|Time|SetTimerbyEvent (delegate Custom|SpawnProjectileVFX) (Variables|Default|GetProjectileSpawnGap) true))

(fn ConstructionScript)